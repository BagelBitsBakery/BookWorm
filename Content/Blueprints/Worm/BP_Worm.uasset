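; BP_Worm is a worm actor with a skeletal mesh that is partly physics-simulated and has an animated eating effect.
; On BeginPlay it enables physics simulation on Bone_001 and all bodies below it.
; The EatEffect event casts the mesh's anim instance to WormEat and plays the EatVal timeline from the start.
; Each timeline update remaps EatLerp into the anim instance's EatValue, leaving the visual result to that animation blueprint.
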(event `self.ReceiveBeginPlay`
  (`SkeletalMeshComponent.SetAllBodiesBelowSimulatePhysics` (`self.SkeletalMesh`) "Bone_001" true true))

(event `self.EatEffect`
  (bind _asworm_eat (cast `/Game/Blueprints/Animations/WormEat` (`SkeletalMeshComponent.GetAnimInstance` (`self.SkeletalMesh`))))
  (set `self.AnimPrint` _asworm_eat)
  (bind (_direction _eatlerp) (`Timeline|EatVal` :!via `PlayFromStart`)
    (:`Update`
      (set `/Game/Blueprints/Animations/WormEat.EatValue` (`KismetMathLibrary.Lerp` -1.0 6.0 _eatlerp) (`self.AnimPrint`)))))

(fn `UserConstructionScript`)